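; Enemy homing missile projectile that steers toward the nearest actor tagged "Homing" and destroys itself after a timed lifetime.
; On BeginPlay it spawns a BP_PlayerExplosion at its transform, then repeatedly calls HeatSeaking on a short delay loop to retarget ProjectileMovement.
; HomingTargetFunction scans tagged actors against a stored CloseDistance, which is never reset between scans, and returns the chosen target's scene component.
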(event Custom|HeatSeaking
  (bind _projectilemovement (Variables|Default|GetProjectileMovement))
  (bind _homing_target (CallFunction|HomingTargetFunction))
  (Variables|/Script/Engine.ProjectileMovementComponent|SetHomingTargetComponent _projectilemovement _homing_target)
  (Variables|/Script/Engine.ProjectileMovementComponent|SetbIsHomingProjectile _projectilemovement true)
  (Utilities|FlowControl|Delay 5.0)
  (Actor|DestroyActor))

(event EventBeginPlay
  (Game|SpawnActorfromClass "/Game/Particles/BP_PlayerExplosion.BP_PlayerExplosion_C" (Transformation|GetActorTransform) "Undefined" "MultiplyWithRoot" 0 0)
  (CallFunction|HeatSeaking :!label _label)
  (Utilities|FlowControl|Delay 0.2)
  (goto _label))

(fn ConstructionScript
  (|CallParentFunction))

(fn HomingTargetFunction
  (bind _outactors (Actor|GetAllActorsOfClasswithTag "/Script/Engine.Actor" "Homing"))
  (for _array_element _outactors
    (if (< (Math|Vector|VectorLength (- (Transformation|GetActorLocation _array_element) (Transformation|GetActorLocation))) (Variables|Default|GetClose%20Distance))
      (Variables|Default|SetClose%20Distance (Math|Vector|VectorLength (- (Transformation|GetActorLocation _array_element) (Transformation|GetActorLocation))))
      (Variables|Default|SetCurrent%20Homing%20Target _array_element)))
  (return (Actor|GetComponentbyClass (Variables|Default|GetCurrent%20Homing%20Target) "/Script/Engine.SceneComponent")))