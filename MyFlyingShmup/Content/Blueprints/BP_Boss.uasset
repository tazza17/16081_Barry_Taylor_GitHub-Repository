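; Boss enemy with a widget health bar that damages any actor overlapping it by its own max health.
; Incoming damage lowers health, updates the bar and briefly flashes an overlay material on all static meshes.
; At zero health it triggers camera shake and adds score via MyPlayerController, spawns death FX, plays sounds and destroys itself.
; An optional pickup, configured through AssignSpawnedEnemyProps, also spawns on death.
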(event Custom|ApplyDamage
  (params (Damage :type Float%20%28double-precision%29))
  ;[0.4072 0 0 1 33] Damage System
  ;;[0.159 0 0] amount of Damage applied to the Enemy
  (Variables|Default|SetHealth (- (Variables|Default|GetHealth) Damage))
  ;[0.009134 0.1878 0.016 1 33] Health System
  ;;[0 1 0.01148] HealthBar System Imported to the Enemy
  (bind _aswbp_boss_health_bar (Utilities|Casting|CastToWBP_BossHealthBar (UserInterface|GetWidget (Variables|Default|GetWidget))))
  (Default|SetBigHealth _aswbp_boss_health_bar (/ (Variables|Default|GetHealth) (Variables|Default|GetMaxHealth))))

(event EventAssignSpawnedEnemyProps
  (params (SpawnPickupOnDeath :type Boolean) (PickUpTypeToSpawn :type BP%20Base%20Pickup%20Class%20Reference))
  ;[0.01764 0 0.05127 1 33] SpawnPickup Event
  (Variables|Default|SetSpawnPickupOnDeath SpawnPickupOnDeath)
  (Variables|Default|SetPickUpTypeToSpawn PickUpTypeToSpawn))

(event Game|Damage|EventAnyDamage
  (params (Damage :type Float%20%28single-precision%29) (DamageType :type Damage%20Type%20Object%20Reference) (InstigatedBy :type Controller%20Object%20Reference) (DamageCauser :type Actor%20Object%20Reference))
  ;[0.4072 0 0 1 33] Damage System
  ;;[0.159 0 0] Applied Damage sequence to the Enemies
  (CallFunction|ApplyDamage Damage)
  ;[0.009134 0.1878 0.016 1 33] Health System
  ;;[0 1 0.01148] Check if Enemy Health = Zero. if so, start Death Sequence
  (if (<= (Variables|Default|GetHealth) 0.0)
    ;[0.3344 0 0.3438 1 33] Sound System with Bullet fire and Bullet contact with the Enemy
    (Audio|PlaySound2D "/Game/Sci-Fi_Shots_Pack2_Game_Of_Weapons/Wave/Cue/SciFi_Shot_P2__102__Cue.SciFi_Shot_P2__102__Cue" 7.0 1.0 0.0 0 0)
    (Utilities|FlowControl|Sequence
      (:then_0
        ;[0 0.2782 1 0.5 33] Camera Shake From MyPlayerController executed when Enemies have Been Killed
        (bind _asmy_player_controller (Utilities|Casting|CastToMyPlayerController (Game|GetPlayerController 0)))
        (Default|ApplyCamShake _asmy_player_controller)
        (Default|AddtoScoreNew _asmy_player_controller (Variables|Default|GetScoredPoints)))
      (:then_1
        ;[1 0.1698 0 0.5] FX Explosion Particles Executed on Enemy Death Sequence
        (Game|SpawnActorfromClass "/Game/Particles/BP_EnemyDeath.BP_EnemyDeath_C" (Math|Transform|MakeTransform (Transformation|GetActorLocation) "0, 0, 0" "1.000000,1.000000,1.000000") "AlwaysSpawn" "MultiplyWithRoot" 0 0)
        ;[0.04959 0 0.15 0.5 33] Pickups Spawning on Enemy Death
        (if (Variables|Default|GetSpawnPickupOnDeath)
          (Game|SpawnActorfromClass (Variables|Default|GetPickUpTypeToSpawn) (Transformation|GetActorTransform) "AlwaysSpawn" "MultiplyWithRoot" 0 0)))
      (:then_2
        (Game|SpawnActorfromClass "/Game/Particles/BP_EnemyDeath.BP_EnemyDeath_C" (Math|Transform|MakeTransform (Transformation|GetActorLocation) "0, 0, 0" "1.000000,1.000000,1.000000") "AlwaysSpawn" "MultiplyWithRoot" 0 0))
      (:then_3
        (Actor|DestroyActor)
        ;[0.3344 0 0.3438 1 33] Enemy Death Sound Effect
        (Audio|PlaySound2D "/Game/Sci-Fi_Shots_Pack2_Game_Of_Weapons/PersonalisedSoundEffects/PointSoundEffect.PointSoundEffect" 1.7 1.0 0.0 0 0)))
    (else
      (Audio|PlaySound2D "/Game/Sci-Fi_Shots_Pack2_Game_Of_Weapons/Wave/Cue/SciFi_Shot_P2__103__Cue.SciFi_Shot_P2__103__Cue" 2.0 1.0 0.0 0 0)
      ;[0.006879 0 0.15 0.5 33] Material Overlay sequence when Enemies are Hit
      (for _array_element (Actor|GetComponentsByClass "/Script/Engine.StaticMeshComponent")
        (Rendering|Material|SetOverlayMaterial _array_element "/Game/materials/MI_DamageFlash.MI_DamageFlash" :!class /Script/Engine.MeshComponent))
      (Utilities|FlowControl|Delay 0.2)
      (for _array_element_2 (Actor|GetComponentsByClass "/Script/Engine.StaticMeshComponent")
        (Rendering|Material|SetOverlayMaterial _array_element_2 0 :!class /Script/Engine.MeshComponent))
      (Utilities|FlowControl|Delay 0.2))))

(event Collision|EventActorBeginOverlap
  (params (OtherActor :type Actor%20Object%20Reference))
  ;[0.4072 0 0 1 33] Damage System
  ;;[0.159 0 0] closer = More damage to player
  (Game|Damage|ApplyDamage OtherActor (Variables|Default|GetMaxHealth) 0 0))

(event EventBeginPlay
  ;[0.009134 0.1878 0.016 1 33] Health System
  ;;[0 1 0.01148] Enemies Assigned Health = +100 Health
  (Variables|Default|SetHealth (Variables|Default|GetMaxHealth)))

(fn ConstructionScript)