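; Enemy spawner Blueprint that repeatedly spawns random enemy types from a class pool at random intervals.
; A timer starts at BeginPlay and is re-queued with a new delay after each spawn.
; Enemies spawn at a random point on a start spline, facing one on an end spline, and receive a random pickup-on-death flag and type.
; All randomness uses one stream seeded with zero.
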(event Custom|SpawnEnemy
  ;[0.15 0.15 0.15 0.5] Starting and End Location Spawn Points
  (bind (_startlocation _endlocation) (CallFunction|GetStartandEndLocation))
  (bind _returnvalue (Game|SpawnActorfromClass (.OutItem (Utilities|Array|RandomFromStream (Variables|Default|GetEnemyClassPool) (Variables|Default|GetRandomStream))) (Math|Transform|MakeTransform _startlocation (Math|Rotator|FindLookatRotation _startlocation _endlocation) "1.000000,1.000000,1.000000") "Undefined" "MultiplyWithRoot" 0 0))
  (Class|BPIMyFlyingShmup|AssignSpawnedEnemyProps(Message) _returnvalue (Class|KismetMathLibrary|RandomBoolwithWeightfromStream (Variables|Default|GetRandomStream) 0.5) (.OutItem (Utilities|Array|RandomFromStream (Variables|Default|GetPickUpClassPool) (Variables|Default|GetRandomStream))))
  (CallFunction|QueueEnemySpawn))

(event Custom|QueueEnemySpawn
  ;[0.15 0.15 0.15 0.5] range of random Spawns
  (bind _returnvalue (Utilities|Time|SetTimerbyEvent (delegate Custom|SpawnEnemy) (Math|Random|RandomFloatinRangefromStream (Variables|Default|GetRandomStream) 1.0 5.0) true true))
  (Variables|Default|SetEnemySpawnTimer _returnvalue))

(event EventBeginPlay
  ;[0.15 0.15 0.15 0.5] Set Random Enemy Spawns - Random Spawn Locations
  (Math|Random|SetRandomStreamSeed (Variables|Default|GetRandomStream) 0)
  (CallFunction|QueueEnemySpawn))

(fn ConstructionScript)

(fn GetStartandEndLocation
  (bind _randomstream (Variables|Default|GetRandomStream))
  (bind _returnvalue (Math|Random|RandomFloatfromStream _randomstream))
  (return (Spline|GetLocationatTime (Variables|Default|GetStartLocation) _returnvalue "World" false) (Spline|GetLocationatTime (Variables|Default|GetEndLocation) _returnvalue "World" false)))