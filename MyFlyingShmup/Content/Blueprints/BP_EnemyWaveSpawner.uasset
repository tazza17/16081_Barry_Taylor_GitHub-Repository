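; Enemy wave spawner that plays through the waves in a WaveData asset, starting at BeginPlay if that asset is valid.
; A timer waits out each wave's initial delay, then StartWave loops over its members with a Delay before each spawn.
; Each spawned enemy receives its pickup-drop settings through a message call.
; After the last member, the wave index increments and the timer re-arms, with no check for the final wave.
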(event Custom|StartWave
  (bind _currentwaveindex (Variables|Default|GetCurrentWaveIndex))
  (bind _wavedata (Variables|Default|GetWaveData))
  (bind _setofwaves (Variables|/Game/framework/PDA_SetOfWaves.PDA_SetOfWaves_C|GetSetOfWaves _wavedata))
  (bind _output (Utilities|Array|Get(acopy) _setofwaves _currentwaveindex))
  ;[0.15 0.15 0.15 0.5] Timer finished = Start Wave
  (Development|PrintString "Starting Wave")
  ;[0.15 0.15 0.15 0.5] Sets to Zero on Start
  (bind _output_get (Variables|Default|SetEnemyMemberIndex 0))
  ;[0.15 0.15 0.15 0.5] True Sends to timer
  ; False Spawns Enemy Class
  (if (> _output_get (Utilities|Array|LastIndex (.enemymembers _output))) :!label _label
    (Math|Integer|IncrementInt (Variables|Default|GetCurrentWaveIndex)
      (:%20%20
        ;[0.15 0.15 0.15 0.5] Time to be Spawned
        (Utilities|Time|SetTimerbyEvent (delegate Custom|StartWave) (.initialwavedelay (Utilities|Array|Get(acopy) (Variables|/Game/framework/PDA_SetOfWaves.PDA_SetOfWaves_C|GetSetOfWaves (stale EventBeginPlay _wavedata)) (Variables|Default|GetCurrentWaveIndex))))
        (Development|PrintString "Waiting for wave")))
    (else
      (Development|PrintString "Waiting for next enemy to spawn")
      ;[0.15 0.15 0.15 0.5] Timed to Wait
      (Utilities|FlowControl|Delay (.initialspawndelay (Utilities|Array|Get(acopy) (.enemymembers _output) (Variables|Default|GetEnemyMemberIndex))))
      ;[0.15 0.15 0.15 0.5] Spawns Chosen Class of Enemies
      (bind _returnvalue (Game|SpawnActorfromClass (.enemyclass (Utilities|Array|Get(acopy) (.enemymembers _output) (Variables|Default|GetEnemyMemberIndex))) (.spawntransform (Utilities|Array|Get(acopy) (.enemymembers _output) (Variables|Default|GetEnemyMemberIndex))) "Undefined" "MultiplyWithRoot" 0 0))
      ;[0.15 0.15 0.15 0.5] Enemy attributes
      (Class|BPIMyFlyingShmup|AssignSpawnedEnemyProps(Message) _returnvalue (.shoulddroppickup (Utilities|Array|Get(acopy) (.enemymembers _output) (Variables|Default|GetEnemyMemberIndex))) (.pickupclass (Utilities|Array|Get(acopy) (.enemymembers _output) (Variables|Default|GetEnemyMemberIndex))))
      ;[0.15 0.15 0.15 0.5] continues the loop = Sent to delay Start all over again
      (Math|Integer|IncrementInt (Variables|Default|GetEnemyMemberIndex)
        (:%20%20
          (goto _label))))))

(event EventBeginPlay
  ;[0.15 0.15 0.15 0.5] checks if Asset is Valid when Played
  (bind _wavedata (Variables|Default|GetWaveData)
    (:then
      ;[0.15 0.15 0.15 0.5] Time to be Spawned
      (Utilities|Time|SetTimerbyEvent (delegate Custom|StartWave) (.initialwavedelay (Utilities|Array|Get(acopy) (Variables|/Game/framework/PDA_SetOfWaves.PDA_SetOfWaves_C|GetSetOfWaves _wavedata) (Variables|Default|GetCurrentWaveIndex))))
      (Development|PrintString "Waiting for wave"))
    (:else)))

(fn ConstructionScript)