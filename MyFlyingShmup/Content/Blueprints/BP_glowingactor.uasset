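; BP_glowingactor is a glowing actor that acts like a timed bomb, dealing radial damage and destroying itself.
; Two seconds after BeginPlay, a timeline's first update tints its point light from green toward yellow, calls SpawnActor with no class set, applies damage and destroys the actor.
; An unconnected chain holds a longer staged countdown through yellow, orange and red that would spawn BP_BombBlast before the same damage and destruction.
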(event EventBeginPlay
  (Utilities|FlowControl|Delay 2.0)
  (bind _colouraplha (Timeline|LightUpTimeLine Play)
    (:Update
      (Rendering|Components|Light|SetLightColor (Variables|Default|GetPointLight) (Math|Color|Lerp(LinearColor) "(R=0.223228,G=1.000000,B=0.000000,A=1.000000)" "(R=1.000000,G=0.990203,B=0.000000,A=1.000000)" _colouraplha) false)
      (Game|SpawnActorfromClass "/Game/Particles/BP_BombBlast.BP_BombBlast_C" (Transformation|GetActorTransform) "Undefined" "MultiplyWithRoot" 0 0)
      (bind _output_get (Variables|Default|SetBaseDamage 5e+01))
      (Game|Damage|ApplyRadialDamage _output_get (Transformation|GetActorLocation) 5e+02 0 0 0 0 false "ECC_Visibility")
      (Actor|DestroyActor))))

(fn ConstructionScript)