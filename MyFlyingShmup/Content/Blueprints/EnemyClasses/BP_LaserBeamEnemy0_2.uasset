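; Laser beam enemy that slides into the play area, fires a single beam, then blows itself up.
; On BeginPlay a timeline sweeps it along negative X from its spawn location.
; Delays chained off the timeline's Update time the attack: after five seconds it spawns the beam projectile at LaserSpawnPoint with a blast sound.
; One second later it spawns BP_PlayerExplosion at its location and destroys itself.
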(event Custom|EnterPlayArea
  (Variables|Default|SetInitialLocation (Transformation|GetActorLocation))
  ;[0.15 0.15 0.15 0.5] Direction and Time to Get to Point A to Point B
  (bind _x_offset (Timeline|TL_EnterPlayArea PlayFromStart)
    (:Update
      (Transformation|SetActorLocation (+ (Variables|Default|GetInitialLocation) (Math|Vector|MakeVector (* _x_offset -1e+04) 0.0 0.0)) true false)
      (Utilities|FlowControl|Delay 5.0)
      (Game|SpawnActorfromClass "/Game/Blueprints/projectileClasses/BP_EnemyLaserBeamprojectile.BP_EnemyLaserBeamprojectile_C" (Transformation|GetWorldTransform (Variables|Default|GetLaserSpawnPoint)) "Undefined" "MultiplyWithRoot" 0 0)
      (Audio|PlaySound2D "/Game/Sci-Fi_Shots_Pack2_Game_Of_Weapons/PersonalisedSoundEffects/MegaBeamSoundBlast.MegaBeamSoundBlast" 0.1 2.0 0.0 0 0)
      (Utilities|FlowControl|Delay 1.0)
      (Game|SpawnActorfromClass "/Game/Particles/BP_PlayerExplosion.BP_PlayerExplosion_C" (Math|Transform|MakeTransform (Transformation|GetActorLocation) "0, 0, 0" "1.000000,1.000000,1.000000") "Undefined" "MultiplyWithRoot" 0 0)
      (Actor|DestroyActor))))

(event EventBeginPlay
  (|CallParentFunction)
  (CallFunction|EnterPlayArea))

(event Collision|EventActorBeginOverlap
  (params (OtherActor :type Actor%20Object%20Reference))
  (|CallParentFunction OtherActor) ; This node is disabled and will not be called.\nDrag off pins to build functionality.
)

(fn ConstructionScript
  (|CallParentFunction))