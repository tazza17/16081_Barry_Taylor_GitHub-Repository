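; Boss enemy Blueprint that scripts the first boss's entrance into the play area and its lateral movement.
; After the parent BeginPlay, a timeline slides it along negative X from its starting location.
; When that finishes, it re-records its location and runs a slowed timeline that offsets it along Y.
; Both moves set the actor location with sweep enabled, scaling timeline curves into world offsets.
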(event Custom|EnterPlayArea
  (Variables|Default|SetInitialLocation (Transformation|GetActorLocation))
  ;[0.15 0.15 0.15 0.5] Direction and Time to Get to Point A to Point B
  (bind _x_offset (Timeline|TL_EnterPlayArea PlayFromStart)
    (:Update
      (Transformation|SetActorLocation (+ (Variables|Default|GetInitialLocation) (Math|Vector|MakeVector (* _x_offset -3e+03) 0.0 0.0)) true false))
    (:Finished
      ;[0.15 0.15 0.15 0.5] After Enemy Enters
      (CallFunction|MoveSidetoSide))))

(event Custom|moveSideToSide
  (Variables|Default|SetInitialLocation (Transformation|GetActorLocation))
  ;[0.15 0.15 0.15 0.5] Speed
  (Components|Timeline|SetPlayRate (Variables|Default|GetTL_MoveSideToSide) 0.4)
  ;[0.15 0.15 0.15 0.5] direction and Time to get to Point A to Point B
  (bind _y_value (Timeline|TL_MoveSideToSide PlayFromStart)
    (:Update
      (Transformation|SetActorLocation (+ (Variables|Default|GetInitialLocation) (Math|Vector|MakeVector 0.0 (* _y_value 4e+03) 0.0)) true false))))

(event EventBeginPlay
  (|CallParentFunction)
  (CallFunction|EnterPlayArea))

(event Collision|EventActorBeginOverlap
  (params (OtherActor :type Actor%20Object%20Reference))
  (|CallParentFunction OtherActor) ; This node is disabled and will not be called.\nDrag off pins to build functionality.
)

(fn ConstructionScript
  (|CallParentFunction))