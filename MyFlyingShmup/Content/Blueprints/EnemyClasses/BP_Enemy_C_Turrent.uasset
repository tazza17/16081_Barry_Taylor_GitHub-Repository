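; BP_Enemy_C_Turrent is a turret enemy that continuously aims at the player and fires bullets automatically.
; Each tick it yaws TurretBase toward the first player pawn using a look-at rotation, with pitch and roll held at zero.
; A looping timer started on BeginPlay spawns BP_Turret_Bullet at BulletSpawnPoint at a fixed interval, with no range or line-of-sight check.
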(event Custom|ShootBullet
  ;[0.15 0.15 0.15 0.5] Turrent Bullet Fire System
  (Game|SpawnActorfromClass "/Game/Blueprints/projectileClasses/BP_Turret_Bullet.BP_Turret_Bullet_C" (Transformation|GetWorldTransform (Variables|Default|GetBullet%20Spawn%20Point)) "AlwaysSpawn" "MultiplyWithRoot" 0 0))

(event EventTick
  (params (DeltaSeconds :type Float%20%28single-precision%29))
  ;[0.15 0.15 0.15 0.5] Turret target System will Always follow the Player / Heat seaking
  (Transformation|SetWorldRotation (Variables|Default|GetTurretBase) (Math|Rotator|MakeRotator 0.0 0.0 (.yaw (Math|Rotator|FindLookatRotation (Transformation|GetActorLocation) (Transformation|GetActorLocation (Game|Player|GetPlayerPawn 0))))) false false))

(event EventBeginPlay
  ;[0.15 0.15 0.15 0.5] Bullet Fire Delayed. Speed per fire
  (|CallParentFunction)
  (Utilities|Time|SetTimerbyEvent (delegate Custom|ShootBullet) 1.0 true true))

(fn ConstructionScript
  (|CallParentFunction))