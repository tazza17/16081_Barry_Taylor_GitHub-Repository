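; BP_Enemy_B_HommingEnemy is an enemy that chases the player while firing bullets.
; Every tick it feeds the direction toward player pawn 0 into FloatingPawnMovement as input and sets its rotation using the look-at yaw.
; On BeginPlay it runs the parent logic, then starts a looping timer that spawns BP_HomingEnemy_Bullet at the BulletSpawn transform with a 2D sound effect.
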(event Custom|ShootBullet
  ;[1 0.1651 0 0.5] Shooting System for Homing Enemies
  (Game|SpawnActorfromClass "/Game/Blueprints/projectileClasses/BP_HomingEnemy_Bullet.BP_HomingEnemy_Bullet_C" (Transformation|GetWorldTransform (Variables|Default|GetBulletSpawn)) "AlwaysSpawn" "MultiplyWithRoot" 0 0)
  ;[1 0.349 0.9134 0.5] Sound Effect
  (Audio|PlaySound2D "/Game/Sci-Fi_Shots_Pack2_Game_Of_Weapons/PersonalisedSoundEffects/EnemyB_Bullet_Sound_Effect.EnemyB_Bullet_Sound_Effect" 0.5 0.7 0.0 0 0))

(event EventTick
  (params (DeltaSeconds :type Float%20%28single-precision%29))
  (bind _returnvalue (Transformation|GetActorLocation))
  (bind _returnvalue_2 (Game|Player|GetPlayerPawn 0))
  (bind _returnvalue_3 (Transformation|GetActorLocation _returnvalue_2))
  ;[0 0.3484 1 0.5] Takes Vector as the Homing Enemies Direction
  (Class|PawnMovementComponent|AddInputVector (Variables|Default|GetFloatingPawnMovement) (Math|Vector|GetUnitDirection(Vector) _returnvalue _returnvalue_3) false)
  ;[1 0.7544 0 0.5] Pointed to the Player. The homing Enemy will follow the player
  (Transformation|SetActorRotation (Math|Rotator|MakeRotator 0.0 0.0 (.yaw (Math|Rotator|FindLookatRotation _returnvalue _returnvalue_3)))))

(event EventBeginPlay
  ;[1 0.1651 0 0.5] Delayed Shooting System changing bullet firing speed
  (|CallParentFunction)
  (Utilities|Time|SetTimerbyEvent (delegate Custom|ShootBullet) 0.6 true true))

(fn ConstructionScript
  (|CallParentFunction))