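; BP_YellowBomb is a homing bomb enemy that chases the player and explodes on a timed fuse.
; Tick drives FloatingPawnMovement toward the player pawn and turns the actor's yaw to face it.
; From BeginPlay, chained timelines and delays shift the LightDetection color green to yellow, orange, then red, each stage triggered from the previous timeline's Update.
; After a final delay it spawns BP_BombBlast at its transform and destroys itself, regardless of player proximity.
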(event EventTick
  (params (DeltaSeconds :type Float%20%28single-precision%29))
  (bind _returnvalue (Transformation|GetActorLocation))
  (bind _returnvalue_2 (Game|Player|GetPlayerPawn 0))
  (bind _returnvalue_3 (Transformation|GetActorLocation _returnvalue_2))
  ;[0 0.3484 1 0.5] Takes Vector as the Homing Enemies Direction
  (Class|PawnMovementComponent|AddInputVector (Variables|Default|GetFloatingPawnMovement) (Math|Vector|GetUnitDirection(Vector) _returnvalue _returnvalue_3) false)
  ;[1 0.7544 0 0.5] Pointed to the Player. The homing Enemy will follow the player
  (Transformation|SetActorRotation (Math|Rotator|MakeRotator 0.0 0.0 (.yaw (Math|Rotator|FindLookatRotation _returnvalue _returnvalue_3)))))

(event EventBeginPlay
  ;[0 1 0.06328 0.5 33] Light Detection System
  (Utilities|FlowControl|Delay 2.0)
  (bind _detection (Timeline|TL_Green,%20Yellow Play)
    (:Update
      (Rendering|Components|Light|SetLightColor (Variables|Default|GetLightDetection) (Math|Color|Lerp(LinearColor) "(R=0.223228,G=1.000000,B=0.000000,A=1.000000)" "(R=1.000000,G=0.990203,B=0.000000,A=1.000000)" _detection) false)
      (Utilities|FlowControl|Delay 5.0)
      (bind _detection_2 (Timeline|TL_Yellow,%20Orange Play)
        (:Update
          (Rendering|Components|Light|SetLightColor (Variables|Default|GetLightDetection) (Math|Color|Lerp(LinearColor) "(R=1.000000,G=0.991102,B=0.000000,A=1.000000)" "(R=1.000000,G=0.245484,B=0.000000,A=1.000000)" _detection_2) false)
          (Utilities|FlowControl|Delay 1e+01)
          (bind _detection_3 (Timeline|TL_Orange,%20Red Play)
            (:Update
              (Rendering|Components|Light|SetLightColor (Variables|Default|GetLightDetection) (Math|Color|Lerp(LinearColor) "(R=1.000000,G=0.246201,B=0.000000,A=1.000000)" "(R=1.000000,G=0.000000,B=0.010729,A=1.000000)" _detection_3) false)
              ;[1 0 0 0.5 33] Explosion
              (Utilities|FlowControl|Delay 2.0)
              (Game|SpawnActorfromClass "/Game/Particles/BP_BombBlast.BP_BombBlast_C" (Transformation|GetActorTransform) "Undefined" "MultiplyWithRoot" 0 0)
              (Actor|DestroyActor))))))))

(fn ConstructionScript
  (|CallParentFunction))