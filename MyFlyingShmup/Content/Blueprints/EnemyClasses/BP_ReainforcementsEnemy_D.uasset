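; BP_ReainforcementsEnemy_D is a reinforcement-spawning enemy pawn that chases the player and keeps producing baby enemies.
; On its first Tick, a DoOnce spawns two BP_EnemyD_SpawnInSequence actors at its own transform.
; Each Tick it moves toward the player through FloatingPawnMovement and yaws to face them.
; From BeginPlay, an endless delayed loop spawns a BP_babyEnemy at each of three bullet spawn points in turn.
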(event Custom|StartingSequence
  ;[0.614 0 1 0.5] SpawnInSequence
  (Utilities|FlowControl|DoOnce false
    (:Completed
      (Game|SpawnActorfromClass "/Game/Particles/BP_EnemyD_SpawnInSequence.BP_EnemyD_SpawnInSequence_C" (Transformation|GetActorTransform) "Undefined" "MultiplyWithRoot" 0 0)
      (Game|SpawnActorfromClass "/Game/Particles/BP_EnemyD_SpawnInSequence.BP_EnemyD_SpawnInSequence_C" (Transformation|GetActorTransform) "Undefined" "MultiplyWithRoot" 0 0))))

(event EventBeginPlay
  ;[0 0.8992 1 0.5] Shooting Sequence
  (Utilities|FlowControl|Delay 2.5 :!label _label)
  (Game|SpawnActorfromClass "/Game/Blueprints/EnemyClasses/BP_babyEnemy.BP_babyEnemy_C" (Transformation|GetWorldTransform (Variables|Default|GetBulletSpawnPoint)) "Undefined" "MultiplyWithRoot" 0 0)
  (Utilities|FlowControl|Delay 2.5)
  (Game|SpawnActorfromClass "/Game/Blueprints/EnemyClasses/BP_babyEnemy.BP_babyEnemy_C" (Transformation|GetWorldTransform (Variables|Default|GetBulletSpawnPoint1)) "Undefined" "MultiplyWithRoot" 0 0)
  (Utilities|FlowControl|Delay 2.5)
  (Game|SpawnActorfromClass "/Game/Blueprints/EnemyClasses/BP_babyEnemy.BP_babyEnemy_C" (Transformation|GetWorldTransform (Variables|Default|GetBulletSpawnPoint2)) "Undefined" "MultiplyWithRoot" 0 0)
  (Utilities|FlowControl|Delay 0.6)
  (goto _label))

(event EventTick
  (params (DeltaSeconds :type Float%20%28single-precision%29))
  (bind _returnvalue (Transformation|GetActorLocation))
  (bind _returnvalue_2 (Game|Player|GetPlayerPawn 0))
  (bind _returnvalue_3 (Transformation|GetActorLocation _returnvalue_2))
  ;[0 0.3125 1 0.5] Follows the Player
  (CallFunction|StartingSequence)
  (Class|PawnMovementComponent|AddInputVector (Variables|Default|GetFloatingPawnMovement) (Math|Vector|GetUnitDirection(Vector) _returnvalue _returnvalue_3) false)
  (Transformation|SetActorRotation (Math|Rotator|MakeRotator 0.0 0.0 (.yaw (Math|Rotator|FindLookatRotation _returnvalue _returnvalue_3)))))

(fn ConstructionScript
  (|CallParentFunction))