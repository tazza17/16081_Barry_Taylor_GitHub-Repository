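; BP_Enemy_A is an enemy that automatically fires bullets from two spawn points.
; On BeginPlay a looping one-second timer calls ShootBullet, which spawns a BP_Enemy_Bullet at each point's world transform and plays a 2D fire sound.
; The construction script assigns PointMesh to the enemy's static mesh component.
; Firing involves no targeting or condition checks, and the file contains no movement or damage logic.
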(event Custom|ShootBullet
  (Game|SpawnActorfromClass "/Game/Blueprints/projectileClasses/BP_Enemy_Bullet.BP_Enemy_Bullet_C" (Transformation|GetWorldTransform (Variables|Default|GetBulletSpawnPoint1)) "Undefined" "MultiplyWithRoot" 0 0)
  (Audio|PlaySound2D "/Game/Sci-Fi_Shots_Pack2_Game_Of_Weapons/PersonalisedSoundEffects/EnemyA_Fire_.EnemyA_Fire_" 0.4 1.0 1.0 0 0)
  (Game|SpawnActorfromClass "/Game/Blueprints/projectileClasses/BP_Enemy_Bullet.BP_Enemy_Bullet_C" (Transformation|GetWorldTransform (Variables|Default|GetBulletSpawnPoint2)) "Undefined" "MultiplyWithRoot" 0 0))

(event EventBeginPlay
  (Utilities|Time|SetTimerbyEvent (delegate Custom|ShootBullet) 1.0 true true))

(fn ConstructionScript
  (Components|StaticMesh|SetStaticMesh (Variables|Default|GetEnemyAMesh) (Variables|Default|GetPointMesh)))