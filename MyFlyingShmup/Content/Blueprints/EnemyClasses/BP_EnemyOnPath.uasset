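; BP_EnemyOnPath is an enemy Blueprint that moves along its own spline path.
; On BeginPlay it detaches the spline, keeping its world transform, so the path stays put as the actor moves.
; A timeline with play rate set to the inverse of TravelTime feeds spline time, moving the actor with sweep at non-constant velocity, without changing rotation.
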(event EventBeginPlay
  (|CallParentFunction)
  (Transformation|DetachFromComponent (Variables|Default|GetSpline) "KeepWorld" "KeepWorld" "KeepWorld" true)
  ;[0.15 0.15 0.15 0.5] Time to get Point A Point B
  (Components|Timeline|SetPlayRate (Variables|Default|GetTL_MoveAlongSline) (/ 1.0 (Variables|Default|GetTravelTime)))
  (bind _time (Timeline|TL_MoveAlongSline PlayFromStart)
    (:Update
      (Transformation|SetActorLocation (Spline|GetLocationatTime (Variables|Default|GetSpline) _time "World" false) true false))))

(fn ConstructionScript
  (|CallParentFunction))